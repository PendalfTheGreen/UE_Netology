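; Test actor Blueprint that exercises custom events, functions with parameters and debug printing.
; The construction script writes MyName into a TextRender label.
; BeginPlay fires a parameterized event that prints its bool and float in a color picked by the bool, then calls a function that multiplies an integer via a helper and re-fires that event.
; Unconnected leftovers include container operations, a visibility toggle and empty events.
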(event Custom|CustomEvent_0
  (params (In_NewParam :type Boolean) (In_NewParam2 :type Byte) (In_NewParam3 :type Name) (In_NewParam4 :type Float%20%28single-precision%29))
  (Development|PrintString (Utilities|String|Append "Bool =" (Utilities|String|ToString(Boolean) In_NewParam) "float =" (Utilities|String|ToString(Float) In_NewParam4)) true false (Math|Color|SelectColor "(R=0.012500,G=1.000000,B=0.088669,A=1.000000)" "(R=1.000000,G=0.000000,B=0.000000,A=1.000000)" In_NewParam) 5.0)
  (Utilities|FlowControl|Delay 1.0))

(event Custom|CustomEvent_1)

(event EventBeginPlay
  (CallFunction|CustomEvent0 false 0 "None" 0.0)
  (CallFunction|CustomEvent0 true 0 "None" 0.5)
  (Test|NewFunction0 "None" (Utilities|Array|MakeArray true) 1))

(event Collision|EventActorBeginOverlap
  (params (OtherActor :type Actor%20Object%20Reference)))

(event EventTick
  (params (DeltaSeconds :type Float%20%28single-precision%29)))

(fn ConstructionScript
  (Rendering|Components|TextRender|SetText (Variables|Default|GetTextRender) (Utilities|Text|FormatText "My name is {Name}" (Variables|Test|GetMy_Name))))

(fn NewFunction0
  (params (In_Name :type Name) (In_Array :type Array%20of%20Booleans) (In_Integer :type Integer))
  (bind _output (Utilities|Array|Get(acopy) In_Array))
  (Utilities|FlowControl|Sequence
    (:then_0)
    (:then_3
      (if _output
        (LocalVariables|SetL_Int (.OutResult (Test|Multipl In_Integer)))
        (CallFunction|CustomEvent0 _output 0 In_Name (Math|Conversions|ToFloat(Integer) (LocalVariables|GetL_Int)))
        (CallFunction|CustomEvent1)
        (return (LocalVariables|GetL_Int))
        (else
          (return 0))))))

(fn NewFunction1)

(fn Multipl
  (params (InParam :type Integer))
  (return (* InParam 5) true))