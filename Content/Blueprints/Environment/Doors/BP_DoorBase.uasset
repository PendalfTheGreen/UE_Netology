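; BP_DoorBase is a base hinged door the player can open and close through its Interract function.
; A box overlap with BP_ThirdPersonCharacter shows a hint and enables interaction.
; One timeline plays forward or in reverse to yaw DoorRotator up to MaxDoorOpenAngle, ignoring new requests while in progress and setting IsDoorOpen by direction on finish.
; The construction script pre-rotates doors flagged as open.
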(event OnComponentBeginOverlap(BoxCollision)
  (params (OverlappedComponent :type Primitive%20Component%20Object%20Reference) (OtherActor :type Actor%20Object%20Reference) (OtherComp :type Primitive%20Component%20Object%20Reference) (OtherBodyIndex :type Integer) (bFromSweep :type Boolean) (SweepResult :type Hit%20Result%20Structure%20%28by%20ref%29))
  (Utilities|Casting|CastToBP_ThirdPersonCharacter OtherActor)
  (Rendering|SetVisibility (Variables|Default|GetHintScene) true true)
  (Variables|Default|SetIsReadyToInteract true))

(event OnComponentEndOverlap(BoxCollision)
  (params (OverlappedComponent :type Primitive%20Component%20Object%20Reference) (OtherActor :type Actor%20Object%20Reference) (OtherComp :type Primitive%20Component%20Object%20Reference) (OtherBodyIndex :type Integer))
  (Utilities|Casting|CastToBP_ThirdPersonCharacter OtherActor)
  (Rendering|SetVisibility (Variables|Default|GetHintScene) false true)
  (Variables|Default|SetIsReadyToInteract false))

(event Custom|CloseDoor
  ;[1 1 1] Door events
  (if (not (Variables|Default|GetInProgress))
    (if (Variables|DoorConfigure|GetIsDoorOpen)
      (bind (_direction _openprogression) (Timeline|DoorTimeline ReverseFromEnd)
        (:Update
          (Variables|Default|SetInProgress true)
          (Transformation|SetRelativeRotation (Variables|Default|GetDoorRotator) (Math|Rotator|MakeRotator 0.0 0.0 (* (Variables|DoorConfigure|GetMaxDoorOpenAngle) _openprogression)) false false))
        (:Finished
          (Variables|Default|SetInProgress false)
          (switch Utilities|FlowControl|Switch|SwitchonETimelineDirection _direction
            (:Forward
              (Variables|DoorConfigure|SetIsDoorOpen true))
            (:Backward
              (Variables|DoorConfigure|SetIsDoorOpen false))))))))

(event Custom|OpenDoor
  ;[1 1 1] Door events
  (if (not (Variables|Default|GetInProgress))
    (if (not (Variables|DoorConfigure|GetIsDoorOpen))
      (bind (_direction _openprogression) (Timeline|DoorTimeline PlayFromStart)
        (:Update
          (Variables|Default|SetInProgress true)
          (Transformation|SetRelativeRotation (Variables|Default|GetDoorRotator) (Math|Rotator|MakeRotator 0.0 0.0 (* (Variables|DoorConfigure|GetMaxDoorOpenAngle) _openprogression)) false false))
        (:Finished
          (Variables|Default|SetInProgress false)
          (switch Utilities|FlowControl|Switch|SwitchonETimelineDirection _direction
            (:Forward
              (Variables|DoorConfigure|SetIsDoorOpen true))
            (:Backward
              (Variables|DoorConfigure|SetIsDoorOpen false))))))))

(event EventBeginPlay
  (Rendering|SetVisibility (Variables|Default|GetHintScene) false true))

(event Collision|EventActorBeginOverlap
  (params (OtherActor :type Actor%20Object%20Reference)))

(event EventTick
  (params (DeltaSeconds :type Float%20%28single-precision%29)))

(fn ConstructionScript
  (Transformation|AddRelativeRotation (Variables|Default|GetDoorRotator) (Math|Rotator|MakeRotator 0.0 0.0 (Math|Float|SelectFloat (Variables|DoorConfigure|GetMaxDoorOpenAngle) 0.0 (Variables|DoorConfigure|GetIsDoorOpen))) false false))

(fn Interract
  (if (Variables|Default|GetIsReadyToInteract)
    (if (Variables|DoorConfigure|GetIsDoorOpen)
      (CallFunction|CloseDoor)
      (return true)
      (else
        (CallFunction|OpenDoor)
        (return true)))
    (else
      (return false))))