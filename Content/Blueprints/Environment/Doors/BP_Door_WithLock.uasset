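; Door actor variant that adds a toggleable lock and an indicator light to its parent door's behavior.
; It overrides OpenDoor to call the parent only when unlocked, while CloseDoor always passes through to the parent.
; SwitchLock flips the lock state and refreshes the light, which shows red when locked and green when unlocked.
; The Construction Script also refreshes the light so it matches the initial lock state.
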(event EventBeginPlay
  (|CallParentFunction) ; This node is disabled and will not be called.\nDrag off pins to build functionality.
)

(event Collision|EventActorBeginOverlap
  (params (OtherActor :type Actor%20Object%20Reference))
  (|CallParentFunction OtherActor) ; This node is disabled and will not be called.\nDrag off pins to build functionality.
)

(event EventTick
  (params (DeltaSeconds :type Float%20%28single-precision%29))
  (|CallParentFunction DeltaSeconds) ; This node is disabled and will not be called.\nDrag off pins to build functionality.
)

(event EventOpenDoor
  (if (not (Variables|DoorConfigure|GetIsDoorLocked))
    (|CallParentFunction)))

(event EventCloseDoor
  (|CallParentFunction))

(fn ConstructionScript
  (|CallParentFunction)
  (CallFunction|UpdateDoorLockIndication))

(fn SwitchLock
  (Variables|DoorConfigure|SetIsDoorLocked (not (Variables|DoorConfigure|GetIsDoorLocked)))
  (CallFunction|UpdateDoorLockIndication))

(fn UpdateDoorLockIndication
  (Rendering|Components|Light|SetLightColor (Variables|Default|GetLockIndicatorLight) (Math|Color|SelectColor "(R=0.776000,G=0.000000,B=0.000000,A=1.000000)" "(R=0.154183,G=1.000000,B=0.000000,A=1.000000)" (Variables|DoorConfigure|GetIsDoorLocked)) true))