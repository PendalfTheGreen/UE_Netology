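; BP_Tooltip_LookOn is an environment tooltip whose text turns to face the third-person character's camera while the look-at flag is on.
; Beginning an overlap sets the flag if CharacterInBox is valid, and ending any overlap clears it.
; Each tick, after the parent logic, LookingAtPlayerCamera rotates TooltipText toward that character's FollowCamera using a look-at rotation.
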(event EventBeginPlay
  (|CallParentFunction) ; This node is disabled and will not be called.\nDrag off pins to build functionality.
)

(event Collision|EventActorBeginOverlap
  (params (OtherActor :type Actor%20Object%20Reference))
  (|CallParentFunction OtherActor) ; This node is disabled and will not be called.\nDrag off pins to build functionality.
)

(event EventTick
  (params (DeltaSeconds :type Float%20%28single-precision%29))
  (|CallParentFunction DeltaSeconds)
  (CallFunction|LookingatPlayerCamera))

(event EventActorBeginOverlap
  (params (OtherActor :type Actor%20Object%20Reference))
  (|CallParentFunction OtherActor)
  (Variables|Default|GetCharacter%20in%20box
    (:then
      (Variables|Default|SetIsLookAtPlayerCamera true))
    (:else)))

(event EventActorEndOverlap
  (params (OtherActor :type Actor%20Object%20Reference))
  (|CallParentFunction OtherActor)
  (Variables|Default|SetIsLookAtPlayerCamera false))

(fn ConstructionScript
  (|CallParentFunction))

(fn LookingatPlayerCamera
  (if (Variables|Default|GetIsLookAtPlayerCamera)
    (bind _character_in_box (Variables|Default|GetCharacter%20in%20box)
      (:then
        (bind _asthird_person_character (Utilities|Casting|CastToBP_ThirdPersonCharacter _character_in_box))
        (Variables|Default|SetCameraLocation (Transformation|GetWorldLocation (Variables|/Game/Blueprints/Character/BP_ThirdPersonCharacter.BP_ThirdPersonCharacter_C|GetFollowCamera _asthird_person_character)))
        (Transformation|SetWorldRotation (Variables|Default|GetTooltip%20Text) (Math|Rotator|FindLookatRotation (Transformation|GetWorldLocation (Variables|Default|GetTooltip%20Text)) (Variables|Default|GetCameraLocation)) false false))
      (:else))))