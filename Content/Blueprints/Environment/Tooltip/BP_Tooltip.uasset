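; BP_Tooltip is a placeable trigger volume that shows a text tooltip in the world while a character stands inside it.
; Overlap events accept any Character, store or clear it in CharacterInBox, and unhide or hide the TooltipText component.
; The construction script applies the box extent, raises the box by its half-height to sit on the actor origin, and sets the text's location and message from variables.
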(event EventBeginPlay)

(event Collision|EventActorBeginOverlap
  (params (OtherActor :type Actor%20Object%20Reference))
  (bind _ascharacter (Utilities|Casting|CastToCharacter OtherActor))
  (Variables|Default|SetCharacter%20in%20box _ascharacter)
  (Development|SetHiddeninGame (Variables|Default|GetTooltip%20Text) false false))

(event EventTick
  (params (DeltaSeconds :type Float%20%28single-precision%29)))

(event Collision|EventActorEndOverlap
  (params (OtherActor :type Actor%20Object%20Reference))
  (Utilities|Casting|CastToCharacter OtherActor)
  (Variables|Default|SetCharacter%20in%20box 0)
  (Development|SetHiddeninGame (Variables|Default|GetTooltip%20Text) true false))

(fn ConstructionScript
  (Components|Box|SetBoxExtent (Variables|Default|GetBoxCollision) (Variables|ToolTipSettings|GetBox%20Extent) true)
  (Transformation|SetRelativeLocation (Variables|Default|GetBoxCollision) (Math|Vector|MakeVector 0.0 0.0 (.Z (Math|Vector|BreakVector (Variables|ToolTipSettings|GetBox%20Extent)))) false false)
  (Transformation|SetRelativeLocation (Variables|Default|GetTooltip%20Text) (Variables|ToolTipSettings|GetTooltipTextLocation) false false)
  (Rendering|Components|TextRender|SetText (Variables|Default|GetTooltip%20Text) (Variables|ToolTipSettings|GetTooltipTextMessage)))